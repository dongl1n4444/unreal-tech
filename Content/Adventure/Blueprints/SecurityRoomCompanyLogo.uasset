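; Animated company logo actor for the security room, built from three Paper2D sprites.
; One timeline moves two of the sprites along relative position tracks, while the other truncates an index track to switch the third sprite's color between blue, red and green.
; BeginPlay and the construction script are empty, and no node in the graph starts either timeline.
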(event EventBeginPlay)

(fn ConstructionScript)