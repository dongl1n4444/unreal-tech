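; World-space button prompt actor that shows a key icon on a material-driven static mesh when the player is nearby.
; The overlap box unpauses a looping timer that checks whether the player's controller can be used and, optionally, whether the player faces the widget within an angle.
; A timeline scales the icon up, reversing on exit or turning away.
; SetIcon selects the key from a 4x4 atlas packed across RGB channels.
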(event OnComponentBeginOverlap(OverlapBox)
  (params (OverlappedComponent :type Primitive%20Component%20Object%20Reference) (OtherActor :type Actor%20Object%20Reference) (OtherComp :type Primitive%20Component%20Object%20Reference) (OtherBodyIndex :type Integer) (bFromSweep :type Boolean) (SweepResult :type Hit%20Result%20Structure%20%28by%20ref%29))
  ;[1 1 1] Enter Trigger
  (if (Actor|ActorHasTag OtherActor (CallFunction|LIBGetPlayerTag))
    (Variables|Default|SetPlayerActor OtherActor)
    (Utilities|Time|UnpauseTimerbyHandle (Variables|Default|GetCheckTimer))))

(event OnComponentEndOverlap(OverlapBox)
  (params (OverlappedComponent :type Primitive%20Component%20Object%20Reference) (OtherActor :type Actor%20Object%20Reference) (OtherComp :type Primitive%20Component%20Object%20Reference) (OtherBodyIndex :type Integer))
  (bind _playeractor (Variables|Default|GetPlayerActor))
  ;[1 1 1] Exit Trigger
  (Utilities|IsValid _playeractor
    (:Is%20Valid
      (if (== OtherActor _playeractor)
        (Utilities|Time|PauseTimerbyHandle (Variables|Default|GetCheckTimer))
        (Variables|Default|SetShowUpIcon false)
        (bind _scale (Timeline|MaxMinWidget Reverse)
          (:Update
            (Rendering|Material|SetScalarParameterValue (Variables|Default|GetDMI) "Scale" (Math|Float|Clamp(Float) _scale (Variables|Setting|GetMinScale)) :!class /Script/Engine.MaterialInstanceDynamic))
          (:Finished
            (if (not (Variables|Default|GetShowUpIcon))
              (Rendering|Material|SetScalarParameterValue (Variables|Default|GetDMI) "p" 1.0 :!class /Script/Engine.MaterialInstanceDynamic))))))))

(event Custom|CheckPlayer
  (bind _playeractor (Variables|Default|GetPlayerActor))
  (Utilities|IsValid _playeractor
    (:Is%20Valid
      (bind _apccontroller (CallFunction|LIBGetAPCController _playeractor self))
      (bind _canuse (Class|BPIPlayerInterface|CanbeUsedBPI(Message) _apccontroller))
      (if _canuse
        (if (Variables|Setting|GetCheckPlayerDirection)
          (if (<= (Class|KismetMathLibrary|DegAcos (Math|Vector|DotProduct (Transformation|GetActorForwardVector (Variables|Default|GetPlayerActor)) (* (Math|Vector|GetForwardVector (Variables|Default|GetArrow)) -1.0))) (Variables|Setting|GetVisibleAngle))
            (if (not (Variables|Default|GetShowUpIcon)) :!label _label
              (Rendering|Material|SetScalarParameterValue (Variables|Default|GetDMI) "p" 0.0 :!class /Script/Engine.MaterialInstanceDynamic)
              (Variables|Default|SetShowUpIcon true)
              (bind _scale (Timeline|MaxMinWidget PlayFromStart)
                (:Update
                  (Rendering|Material|SetScalarParameterValue (Variables|Default|GetDMI) "Scale" (Math|Float|Clamp(Float) _scale (Variables|Setting|GetMinScale)) :!class /Script/Engine.MaterialInstanceDynamic))
                (:Finished
                  (if (not (Variables|Default|GetShowUpIcon))
                    (Rendering|Material|SetScalarParameterValue (Variables|Default|GetDMI) "p" 1.0 :!class /Script/Engine.MaterialInstanceDynamic)))))
            (elif (Variables|Default|GetShowUpIcon)
              (Variables|Default|SetShowUpIcon false)
              (Timeline|MaxMinWidget Reverse)))
          (else
            (goto _label)))))))

(event Custom|SetIcon
  (params (Key :type E_ButtonWidget%20Enum :default "NewEnumerator0"))
  (bind _returnvalue (Math|Conversions|ToInteger(Byte) Key))
  (bind _dmi (Variables|Default|GetDMI))
  (bind _dmi_2 (Variables|Default|GetDMI))
  (bind _dmi_3 (Variables|Default|GetDMI))
  (bind _returnvalue_2 (Math|Integer|%(Integer) _returnvalue 16))
  ;[1 1 1] SetIcon
  (Rendering|Material|SetScalarParameterValue _dmi_2 "u" (/ (Math|Conversions|ToFloat(Integer) (Math|Integer|%(Integer) _returnvalue_2 4)) 4.0) :!class /Script/Engine.MaterialInstanceDynamic)
  (Rendering|Material|SetScalarParameterValue _dmi_2 "v" (/ (Math|Conversions|ToFloat(Integer) (/ _returnvalue_2 4)) 4.0) :!class /Script/Engine.MaterialInstanceDynamic)
  (Rendering|Material|SetScalarParameterValue _dmi_3 "r" 0.0 :!class /Script/Engine.MaterialInstanceDynamic)
  (Rendering|Material|SetScalarParameterValue _dmi_3 "g" 0.0 :!class /Script/Engine.MaterialInstanceDynamic)
  (Rendering|Material|SetScalarParameterValue _dmi_3 "b" 0.0 :!class /Script/Engine.MaterialInstanceDynamic)
  (switch int (/ _returnvalue 16)
    (:0
      (Rendering|Material|SetScalarParameterValue _dmi "r" 1.0 :!class /Script/Engine.MaterialInstanceDynamic))
    (:1
      (Rendering|Material|SetScalarParameterValue _dmi "g" 1.0 :!class /Script/Engine.MaterialInstanceDynamic))
    (:2
      (Rendering|Material|SetScalarParameterValue _dmi "b" 1.0 :!class /Script/Engine.MaterialInstanceDynamic))))

(event EventBeginPlay
  (Variables|Default|SetHidden false)
  (bind _returnvalue (Rendering|Material|CreateDynamicMaterialInstance (Variables|Default|GetStaticMesh) 0 "/Game/Puzzle/Materials/M_ButtonWidget.M_ButtonWidget" "None" :!class /Script/Engine.PrimitiveComponent))
  (bind _output_get (Variables|Default|SetDMI _returnvalue))
  (Rendering|Material|SetScalarParameterValue _output_get "ParticleWidth" (Variables|Setting|GetWidth) :!class /Script/Engine.MaterialInstanceDynamic)
  (Rendering|Material|SetScalarParameterValue _output_get "ParticleHeight" (* (Variables|Setting|GetHeight) -1.0) :!class /Script/Engine.MaterialInstanceDynamic)
  (Rendering|Material|SetVectorParameterValue _output_get "Color" (Variables|Setting|GetColor) :!class /Script/Engine.MaterialInstanceDynamic)
  (Rendering|Material|SetScalarParameterValue _output_get "Scale" (Variables|Setting|GetMinScale) :!class /Script/Engine.MaterialInstanceDynamic)
  (Rendering|Material|SetScalarParameterValue _output_get "p" 1.0 :!class /Script/Engine.MaterialInstanceDynamic)
  (CallFunction|SetIcon (Variables|Setting|GetKeyIcon))
  (bind _returnvalue_2 (Utilities|Time|SetTimerbyFunctionName self "CheckPlayer" 0.15 true))
  (bind _output_get_2 (Variables|Default|SetCheckTimer _returnvalue_2))
  (Utilities|Time|PauseTimerbyHandle _output_get_2))

(event Collision|EventActorBeginOverlap
  (params (OtherActor :type Actor%20Object%20Reference)))

(event EventTick
  (params (DeltaSeconds :type Float%20%28single-precision%29)))

(fn ConstructionScript
  (Components|Box|SetBoxExtent (Variables|Default|GetOverlapBox) (Variables|Setting|GetOverlapBoxSize) true)
  (Transformation|SetRelativeLocation (Variables|Default|GetStaticMesh) (Variables|Setting|GetWidgetOffset) false false))

(fn GetVisibleAngleBPI
  (return 0.0))

(fn IsWidgetHiddenBPI
  (return false))