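; APC_Library is a Blueprint function library of shared helpers for the puzzle game's APC system.
; It returns the player tag, fetches the APC_Controller component from a player actor and assigns an owner to BP_OverlapWidget child actors.
; An action dispatcher maps Flip Flop to an interface message on the target actor.
; Print String wrappers provide colored log, warning and error output, which the helpers use to report failures.
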(fn LIBGetPlayerTag
  (return "Player"))

(fn LIBGetAPCController
  (params (PlayerActor :type Actor%20Object%20Reference) (Instigator :type Actor%20Object%20Reference))
  (bind _returnvalue (Actor|GetComponentsByClass PlayerActor "/Game/Puzzle/BluePrints/APC_Controller.APC_Controller_C"))
  (bind _output (Utilities|Array|Get(acopy) _returnvalue))
  (Utilities|IsValid _output
    (:Is%20Valid
      (return _output))
    (:Is%20Not%20Valid
      (CallFunction|LIBDebugPrint (Utilities|String|Append (Utilities|GetDisplayName Instigator) "-> Get APC_Controller failed!") "(R=0.000000,G=0.658824,B=1.000000,A=1.000000)" 2.0)
      (return 0))))

(fn LIBDebugPrint
  (params (TextToPrint :type String) (Color :type Linear%20Color%20Structure :default "(R=0.000000,G=0.658824,B=1.000000,A=1.000000)") (Duration :type Float%20%28single-precision%29))
  (Development|PrintString 0 TextToPrint true true Color Duration))

(fn LIBDebugLogError
  (params (Text :type String))
  (CallFunction|LIBDebugPrint (Utilities|String|Append "Error:" Text) "(R=1.000000,G=0.000000,B=0.000000,A=1.000000)" 2.0))

(fn LIBDebugLog
  (params (Text :type String))
  (CallFunction|LIBDebugPrint Text "(R=0.390625,G=0.384192,B=0.375954,A=1.000000)" 2.0))

(fn LIBDebugLogWarning
  (params (Text :type String))
  (CallFunction|LIBDebugPrint (Utilities|String|Append "Warning:" Text) "(R=1.000000,G=1.000000,B=0.000000,A=1.000000)" 2.0))

(fn LIBSetOverlapWidget
  (params (OverlapWidgetComp :type Child%20Actor%20Component%20Object%20Reference) (OverlapWidgetDelegate :type BPI%20Overlap%20Widget%20Delegate%20Interface))
  (bind _asbp_overlap_widget (Utilities|Casting|CastToBP_OverlapWidget (Variables|/Script/Engine.ChildActorComponent|GetChildActor OverlapWidgetComp))
    (:then
      (Variables|/Game/Puzzle/BluePrints/BP_OverlapWidget.BP_OverlapWidget_C|SetOwnerActor _asbp_overlap_widget OverlapWidgetDelegate)
      (return))
    (:CastFailed
      (CallFunction|LIBDebugLogError (Utilities|String|Append (Utilities|GetDisplayName (Utilities|ToObject(Interface) OverlapWidgetDelegate)) "failed cast overlapwidget to bp_overlapwidget"))
      (return))))

(fn LIBExecuteAction
  (params (Actor :type Actor%20Object%20Reference) (Action :type E_Actor_Action%20Enum :default "NewEnumerator9"))
  (Utilities|IsValid Actor
    (:Is%20Valid
      (switch Utilities|FlowControl|Switch|SwitchonE_Actor_Action Action
        (:NewEnumerator17
          (Class|BPIActorAction|FlipFlopBPI(Message) Actor))))
    (:Is%20Not%20Valid
      (CallFunction|LIBDebugLogError "failed execute action because actor is null"))))