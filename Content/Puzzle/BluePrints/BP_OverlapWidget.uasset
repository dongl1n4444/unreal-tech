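; BP_OverlapWidget is a puzzle interactable with a box trigger that registers itself with the player's controller while the player overlaps it.
; On overlap, it checks the player tag and asks the controller through interface messages whether it can be used, then adds itself, removing itself on exit.
; The construction script sizes the box; the interface returns a fixed object type, and its action only prints debug text.
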(event OnComponentBeginOverlap(Overlap)
  (params (OverlappedComponent :type Primitive%20Component%20Object%20Reference) (OtherActor :type Actor%20Object%20Reference) (OtherComp :type Primitive%20Component%20Object%20Reference) (OtherBodyIndex :type Integer) (bFromSweep :type Boolean) (SweepResult :type Hit%20Result%20Structure%20%28by%20ref%29))
  (if (Actor|ActorHasTag OtherActor (CallFunction|LIBGetPlayerTag))
    (bind _output_get (Variables|Default|SetPlayerActor OtherActor))
    (bind _apccontroller (CallFunction|LIBGetAPCController _output_get))
    (bind _canuse (Class|BPIPlayerInterface|CanbeUsedBPI(Message) _apccontroller))
    (if _canuse
      (Class|BPIPlayerInterface|AddOverlappedObjectBPI(Message) _apccontroller self)
      (Variables|Default|SetOverlapAdded true))))

(event OnComponentEndOverlap(Overlap)
  (params (OverlappedComponent :type Primitive%20Component%20Object%20Reference) (OtherActor :type Actor%20Object%20Reference) (OtherComp :type Primitive%20Component%20Object%20Reference) (OtherBodyIndex :type Integer))
  (if (and (Actor|ActorHasTag OtherActor (CallFunction|LIBGetPlayerTag)) (Variables|Default|GetOverlapAdded))
    (bind _apccontroller (CallFunction|LIBGetAPCController OtherActor))
    (Class|BPIPlayerInterface|RemoveOverlappedObjectBPI(Message) _apccontroller self)))

(event EventBeginPlay)

(event Collision|EventActorBeginOverlap
  (params (OtherActor :type Actor%20Object%20Reference)))

(event EventTick
  (params (DeltaSeconds :type Float%20%28single-precision%29)))

(event EventActionOneBPI
  (params (PlayerActor :type Actor%20Object%20Reference))
  (CallFunction|LIBDebugPrint "BP_OverlapWidget.ActionOne" "(R=0.000000,G=0.658824,B=1.000000,A=1.000000)" 2.0))

(fn ConstructionScript
  (Components|Box|SetBoxExtent (Variables|Default|GetOverlap) (Variables|Setting|GetOverlapBoxSize) true))

(fn GetObjectTypeBPI
  (return "NewEnumerator2"))

(fn GetTargetTransformBPI
  (return ""))