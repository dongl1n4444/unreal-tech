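; BP_APC_Player is the player input Blueprint for a puzzle game, passing movement, look and jump controls to an APCController.
; Move, turn, look-up and jump inputs each call a matching function on APCController, so no movement logic lives in these graphs.
; BeginPlay fades the camera in from full opacity through the player camera manager.
; The TurnRate axis event is present but unused, and the construction script is empty.
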(event EventBeginPlay
  ;[1 1 1] FadeIn
  (CameraFades|StartCameraFade :self (Game|GetPlayerCameraManager 0) :FromAlpha 1.0 :Duration 4.0))

(event Input|ActionEvents|InputActionJump
  (params (Key :type Key%20Structure :default "None"))
  (:Pressed
    (Default|JumpInput (Variables|Default|GetAPC_Controller))))

(event Input|AxisEvents|InputAxisTurn
  (params (AxisValue :type Float%20%28single-precision%29))
  (Default|AddYamInput (Variables|Default|GetAPC_Controller) AxisValue))

(event Input|AxisEvents|InputAxisTurnRate
  (params (AxisValue :type Float%20%28single-precision%29)))

(event Input|AxisEvents|InputAxisLookUp
  (params (AxisValue :type Float%20%28single-precision%29))
  (Default|AddPitchInput (Variables|Default|GetAPC_Controller) AxisValue))

(event Input|AxisEvents|InputAxisMoveForward
  (params (AxisValue :type Float%20%28single-precision%29))
  (Default|MoveForwardInput (Variables|Default|GetAPC_Controller) AxisValue))

(event Input|AxisEvents|InputAxisMoveRight
  (params (AxisValue :type Float%20%28single-precision%29))
  (Default|MoveRightInput (Variables|Default|GetAPC_Controller) AxisValue))

(fn ConstructionScript)