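; Small interactable puzzle door that slides between open and closed arrow markers, driven by interface calls or a debug key.
; Requests set flags that Tick consumes to start timelines lerping the door, with a lock against re-triggering mid-move.
; A safety blocker collides until the door is fully open, and audio parameters alternate impact sounds on closing.
; An overlap area registers the door with the player's controller, whose action toggles it.
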(event OnComponentBeginOverlap(OverlapArea)
  (params (OverlappedComponent :type Primitive%20Component%20Object%20Reference) (OtherActor :type Actor%20Object%20Reference) (OtherComp :type Primitive%20Component%20Object%20Reference) (OtherBodyIndex :type Integer) (bFromSweep :type Boolean) (SweepResult :type Hit%20Result%20Structure%20%28by%20ref%29))
  (CallFunction|CheckSetPlayerOverlap OtherActor))

(event OnComponentEndOverlap(OverlapArea)
  (params (OverlappedComponent :type Primitive%20Component%20Object%20Reference) (OtherActor :type Actor%20Object%20Reference) (OtherComp :type Primitive%20Component%20Object%20Reference) (OtherBodyIndex :type Integer))
  (if (and (Actor|ActorHasTag OtherActor (CallFunction|LIBGetPlayerTag)) (Variables|Default|GetOverlapAdded))
    (bind _apccontroller (CallFunction|LIBGetAPCController OtherActor))
    (Class|BPIPlayerInterface|RemoveOverlappedObjectBPI(Message) _apccontroller self)))

(event Custom|EnableSaftyBlocker
  (params (Enable :type Boolean))
  (bind _saftyblocker (Variables|Default|GetSaftyBlocker))
  (if Enable
    (Collision|SetCollisionEnabled _saftyblocker "QueryAndPhysics")
    (else
      (Collision|SetCollisionEnabled _saftyblocker "NoCollision"))))

(event Custom|ManagerSound
  (params (Impact :type Boolean))
  (bind _audio (Variables|Default|GetAudio))
  ;[1 1 1] Sound
  (if Impact
    (switch int (Variables|Default|GetImpactCount)
      (:0
        (Effects|Components|ParticleSystem|SetBoolParameter _audio "DoorImpact" true)
        (Math|Integer|IncrementInt (Variables|Default|GetImpactCount)))
      (:1
        (Effects|Components|ParticleSystem|SetBoolParameter _audio "DoorImpact2" true)
        (Variables|Default|SetImpactCount 0)))
    (else
      (Audio|Components|Audio|Play _audio 0.0)
      (Effects|Components|ParticleSystem|SetBoolParameter _audio "DoorImpact" false)
      (Effects|Components|ParticleSystem|SetBoolParameter _audio "DoorImpact2" false))))

(event Custom|CheckSetPlayerOverlap
  (params (Actor :type Actor%20Object%20Reference))
  (if (Actor|ActorHasTag Actor (CallFunction|LIBGetPlayerTag))
    (bind _output_get (Variables|Default|SetPlayerActor Actor))
    (bind _apccontroller (CallFunction|LIBGetAPCController _output_get))
    (bind _canuse (Class|BPIPlayerInterface|CanbeUsedBPI(Message) _apccontroller))
    (if _canuse
      (Class|BPIPlayerInterface|AddOverlappedObjectBPI(Message) _apccontroller self)
      (Variables|Default|SetOverlapAdded true))))

(event EventBeginPlay)

(event Collision|EventActorBeginOverlap
  (params (OtherActor :type Actor%20Object%20Reference)))

(event EventTick
  (params (DeltaSeconds :type Float%20%28single-precision%29))
  (if (Variables|Setting|GetEnabled)
    (if (Variables|Default|GetWantCloseDoor)
      ;[1 1 1] Close
      (Variables|Default|SetWantCloseDoor false)
      (Variables|Default|SetDoor1TargetLocation (Transformation|GetWorldLocation (Variables|Default|GetDoorCloseArrow)))
      (Variables|Default|SetDoor1StartLocation (Transformation|GetWorldLocation (Variables|Default|GetDoor)))
      (CallFunction|ManagerSound true)
      (bind _closedoor (Timeline|时间轴_1 PlayFromStart)
        (:Update
          (Transformation|SetWorldLocation (Variables|Default|GetDoor) (Math|Vector|Lerp(Vector) (Variables|Default|GetDoor1StartLocation) (Variables|Default|GetDoor1TargetLocation) _closedoor) false true))
        (:Finished
          (Variables|Default|SetCloseOpenInProgress false)
          (Variables|Default|SetIsDoorOpen false)
          (CallFunction|EnableSaftyBlocker true)))
      (else
        ;[1 1 1] Open
        (if (Variables|Default|GetWantOpenDoor)
          (Variables|Default|SetWantOpenDoor false)
          (Variables|Default|SetDoor1TargetLocation (Transformation|GetWorldLocation (Variables|Default|GetDoorOpenArrow)))
          (Variables|Default|SetDoor1StartLocation (Transformation|GetWorldLocation (Variables|Default|GetDoor)))
          (CallFunction|ManagerSound false)
          (bind _opendoor (Timeline|时间轴_0 PlayFromStart)
            (:Update
              (Transformation|SetWorldLocation (Variables|Default|GetDoor) (Math|Vector|Lerp(Vector) (Variables|Default|GetDoor1StartLocation) (Variables|Default|GetDoor1TargetLocation) _opendoor) false false))
            (:Finished
              (Variables|Default|SetCloseOpenInProgress false)
              (Variables|Default|SetIsDoorOpen true)
              (CallFunction|EnableSaftyBlocker false))))))))

(event EventOpenBPI
  (if (not (Variables|Default|GetCloseOpenInProgress))
    (if (not (Variables|Default|GetIsDoorOpen))
      (Variables|Default|SetWantOpenDoor true)
      (Variables|Default|SetWantCloseDoor false)
      (Variables|Default|SetCloseOpenInProgress true)
      (CallFunction|EnableSaftyBlocker true))))

(event EventActionOneBPI
  (params (PlayerActor :type Actor%20Object%20Reference))
  (CallFunction|LIBDebugPrint "SMALLDOOR.Action One BPI" "(R=0.000000,G=0.658824,B=1.000000,A=1.000000)" 2.0)
  (CallFunction|FlipFlopBPI))

(event EventFlipFlopBPI
  (if (Variables|Default|GetIsDoorOpen)
    (CallFunction|CloseBPI)
    (else
      (CallFunction|OpenBPI))))

(event EventCloseBPI
  (if (not (Variables|Default|GetCloseOpenInProgress))
    (if (Variables|Default|GetIsDoorOpen)
      (Variables|Default|SetWantOpenDoor false)
      (Variables|Default|SetWantCloseDoor true)
      (Variables|Default|SetCloseOpenInProgress true))))

(event Input|KeyboardEvents|J
  (params (Key :type Key%20Structure :default "None"))
  ;[1 1 1] Debug
  (:Pressed
    (CallFunction|FlipFlopBPI)))

(fn ConstructionScript
  (if (Variables|Setting|GetInitOpenDoor)
    (Transformation|SetWorldLocation (Variables|Default|GetDoor) (Transformation|GetWorldLocation (Variables|Default|GetDoorOpenArrow)) false false)))

(fn GetObjectTypeBPI
  (return "NewEnumerator2"))

(fn GetTargetTransformBPI
  (return (Transformation|GetWorldTransform (Variables|Default|GetPlayerTarget))))